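; BP_ActorReproductor is an actor sketching self-replication, but the replication logic is currently disconnected.
; BeginPlay only runs a short delay with nothing wired after it.
; An unreachable chain would spawn another BP_ActorReproductor at SpawnDistance in a random direction from itself, keeping its rotation, then immediately destroy that new copy.
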(event EventBeginPlay
  (Utilities|FlowControl|Delay 0.2))

(fn ConstructionScript)